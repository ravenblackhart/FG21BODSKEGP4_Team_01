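; Player character Blueprint with a mid-air ground slam that launches boxes on landing.
; Pressing Interact while falling sets a smacking flag, removes air control, raises gravity and squashes the mesh.
; Tick detects the landing, restores those settings, plays a sound and impulses every entry in Boxes away from the player with a strong vertical bias, without a range check.
; The PlayerDeath event only prints a debug message.
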(event EventTick
  (params (DeltaSeconds :type Float%20%28single-precision%29))
  (bind _charactermovement (Variables|Character|GetCharacterMovement))
  (if (and (AI|Components|NavMovement|IsMovingonGround (Variables|Character|GetCharacterMovement)) (Variables|Default|GetisSmacking))
    (Variables|Default|SetisSmacking false)
    (Variables|/Script/Engine.CharacterMovementComponent|SetAirControl _charactermovement 0.35)
    (Variables|/Script/Engine.CharacterMovementComponent|SetGravityScale _charactermovement 1.75)
    (Transformation|SetWorldScale3D (Variables|Character|GetMesh) "1.000000,1.000000,1.000000")
    (Audio|PlaySoundatLocation "/Engine/EditorSounds/Notifications/CompileSuccess.CompileSuccess" "0, 0, 0" "0, 0, 0" 1.0 1.0 0.0 0 0 0 0)
    (for _array_element (Variables|Default|GetBoxes)
      (Physics|AddImpulse (Variables|/Script/Engine.StaticMeshActor|GetStaticMeshComponent _array_element) (* (Math|Vector|Normalize (- (Transformation|GetWorldLocation (Variables|/Script/Engine.StaticMeshActor|GetStaticMeshComponent _array_element)) (Transformation|GetWorldLocation (Variables|Character|GetMesh)))) "5000.000000,5000.000000,100000.000000") "None" false)
      (Development|PrintString "Please don't do that to me"))))

(event EventPlayerDeath
  ;[1 1 1] Player Death
  (Development|PrintString "U DED" true true "(R=1.000000,G=0.000000,B=0.676688,A=1.000000)"))

(event Input|ActionEvents|InputActionInteract
  (params (Key :type Key%20Structure :default "None"))
  (bind _charactermovement (Variables|Character|GetCharacterMovement))
  (:Pressed
    (if (AI|Components|NavMovement|IsFalling _charactermovement)
      (Variables|Default|SetisSmacking true)
      (Variables|/Script/Engine.CharacterMovementComponent|SetAirControl _charactermovement 0.0)
      (Variables|/Script/Engine.CharacterMovementComponent|SetGravityScale _charactermovement 1e+01)
      (Transformation|SetWorldScale3D (Variables|Character|GetMesh) "1.000000,1.000000,0.500000"))))

(fn ConstructionScript)