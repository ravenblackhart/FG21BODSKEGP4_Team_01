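; Enemy character Blueprint that wanders at random and moves toward the player when it sees them.
; From BeginPlay, a wander loop waits a random delay, moves to a reachable nearby point, then repeats, with IsMoving guarding new moves.
; Pawn sensing triggers AIMoveTo toward the player's last updated location; a retriggerable delay resumes wandering once sightings stop, while seeing other pawns resumes it directly.
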(event OnSeePawn(PawnSensing)
  (params (Pawn :type Pawn%20Object%20Reference))
  ;[1 1 1] AI detect player
  (if (== Pawn (Game|GetPlayerCharacter 0))
    (Development|PrintString "Player Seen by enemy" true true "(R=1.000000,G=0.516063,B=0.000000,A=1.000000)")
    ;;[1 0.401 0.401] Follow Player
    (Variables|Default|SetisMoving true)
    (AI|AIMoveTo self (Class|CharacterMovementComponent|GetLastUpdateLocation (Variables|/Script/Engine.Character|GetCharacterMovement (Game|GetPlayerCharacter 0))) 0 5.0 false
      (:then
        (Utilities|FlowControl|RetriggerableDelay 1.0))))
  ;;[0.6885 0.4366 1] Wander again
  (Development|PrintString "Not Player Seen by enemy" true true "(R=1.000000,G=0.169013,B=0.000000,A=1.000000)")
  (Variables|Default|SetisMoving false)
  (CallFunction|AIWander))

(event Custom|AI_Wander
  ;[1 1 1] Wander at random
  (Utilities|FlowControl|Delay (Math|Random|RandomFloatinRange 0.3 3.0))
  (if (Variables|Default|GetisMoving)
    (Development|PrintString "AI is moving" true true "(R=1.000000,G=0.019619,B=0.000000,A=1.000000)")
    (else
      (AI|AIMoveTo self (.RandomLocation (AI|Navigation|GetRandomReachablePointinRadius (Transformation|GetActorLocation) 5e+02 0 0)) 0 5.0 false
        (:then
          (Variables|Default|SetisMoving true))
        (:OnSuccess
          (Variables|Default|SetisMoving false :!label _label)
          (CallFunction|AIWander))
        (:OnFail
          (goto _label))))))

(event Custom|Check_FOV
  ;[1 1 1] AI detect player
  (if (== (stale OnSeePawn(PawnSensing) Pawn) (Game|GetPlayerCharacter 0))
    (Development|PrintString "Player Seen by enemy" true true "(R=1.000000,G=0.516063,B=0.000000,A=1.000000)")
    ;;[1 0.401 0.401] Follow Player
    (Variables|Default|SetisMoving true)
    (AI|AIMoveTo self (Class|CharacterMovementComponent|GetLastUpdateLocation (Variables|/Script/Engine.Character|GetCharacterMovement (Game|GetPlayerCharacter 0))) 0 5.0 false
      (:then
        (Utilities|FlowControl|RetriggerableDelay 1.0))))
  ;;[0.6885 0.4366 1] Wander again
  (Development|PrintString "Not Player Seen by enemy" true true "(R=1.000000,G=0.169013,B=0.000000,A=1.000000)")
  (Variables|Default|SetisMoving false)
  (CallFunction|AIWander))

(event EventBeginPlay
  ;[1 1 1] Wander at random
  (Utilities|FlowControl|Delay (Math|Random|RandomFloatinRange 0.3 3.0))
  (if (Variables|Default|GetisMoving)
    (Development|PrintString "AI is moving" true true "(R=1.000000,G=0.019619,B=0.000000,A=1.000000)")
    (else
      (AI|AIMoveTo self (.RandomLocation (AI|Navigation|GetRandomReachablePointinRadius (Transformation|GetActorLocation) 5e+02 0 0)) 0 5.0 false
        (:then
          (Variables|Default|SetisMoving true))
        (:OnSuccess
          (Variables|Default|SetisMoving false :!label _label)
          (CallFunction|AIWander))
        (:OnFail
          (goto _label))))))

(fn ConstructionScript)