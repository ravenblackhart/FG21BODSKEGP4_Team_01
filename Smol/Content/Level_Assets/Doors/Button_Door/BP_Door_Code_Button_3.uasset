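; Button Blueprint for a code door, acting as button 3 for its DoorTarget.
; Player overlap with TriggerRange enables input and opens a gate; leaving the range disables input.
; The first E press through the gate calls DoorCodeLight3Message on DoorTarget, turns the PointLight green and prints a status string.
; A DoOnce with no reset wired makes the activation one-time.
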(event OnComponentBeginOverlap(Triggerrange)
  (params (OverlappedComponent :type Primitive%20Component%20Object%20Reference) (OtherActor :type Actor%20Object%20Reference) (OtherComp :type Primitive%20Component%20Object%20Reference) (OtherBodyIndex :type Integer) (bFromSweep :type Boolean) (SweepResult :type Hit%20Result%20Structure%20%28by%20ref%29))
  (if (== OtherActor (Game|GetPlayerCharacter 0))
    (Input|EnableInput (Game|GetPlayerController 0))
    (Utilities|FlowControl|Gate true) ; enters at Open
  ))

(event OnComponentEndOverlap(Triggerrange)
  (params (OverlappedComponent :type Primitive%20Component%20Object%20Reference) (OtherActor :type Actor%20Object%20Reference) (OtherComp :type Primitive%20Component%20Object%20Reference) (OtherBodyIndex :type Integer))
  (if (== OtherActor (Game|GetPlayerCharacter 0))
    (Input|DisableInput (Game|GetPlayerController 0))))

(event Input|KeyboardEvents|E
  (params (Key :type Key%20Structure :default "None"))
  (:Pressed
    (Utilities|FlowControl|Gate true
      (:Exit
        (Utilities|FlowControl|DoOnce false
          (:Completed
            (Class|BPIDoors|DoorCodeLight3(Message) (Variables|Default|GetDoor%20target))
            (Rendering|Components|Light|SetLightColor (Variables|Default|GetPointLight) "(R=0.000000,G=1.000000,B=0.000000,A=1.000000)" true)
            (Development|PrintString "Button Active")))))))

(fn ConstructionScript)