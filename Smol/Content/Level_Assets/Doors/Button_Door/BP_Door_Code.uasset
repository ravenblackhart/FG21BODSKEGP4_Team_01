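; BP_Door_Code is a button-operated door that opens once all three of its indicator lights are activated.
; Three custom events each turn their light green and set a matching active flag, then run a shared check.
; When all three flags are true, MoveComponentTo eases the door downward along Z; otherwise it prints a not-pressed message.
; Nothing in the Blueprint resets the flags or lights.
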(event EventDoorCodeLight1
  (Rendering|Components|Light|SetLightColor (Variables|Default|GetLight_1) (Utilities|Struct|MakeLinearColor 0.0 1.0 0.0 0.0) true)
  (bind _output_get (Variables|Default|SetLight_active_1 true))
  (if (Math|Boolean|ANDBoolean _output_get (stale EventDoorCodeLight2 _output_get) (stale EventDoorCodeLight3 _output_get))
    (Components|MoveComponentTo (Variables|Default|GetDoor) (- (Variables|/Script/Engine.SceneComponent|GetRelativeLocation (Variables|Default|GetDoor)) "0,0,500.000000") "0, 0, 0" true true 3.0 false)
    (else
      (Development|PrintString "Buttons not Pressed"))))

(event EventDoorCodeLight2
  (Rendering|Components|Light|SetLightColor (Variables|Default|GetLight_2) (Utilities|Struct|MakeLinearColor 0.0 1.0 0.0 0.0) true)
  (bind _output_get (Variables|Default|SetLight_active_2 true))
  (if (Math|Boolean|ANDBoolean (stale EventDoorCodeLight1 _output_get) _output_get (stale EventDoorCodeLight3 _output_get))
    (Components|MoveComponentTo (Variables|Default|GetDoor) (- (Variables|/Script/Engine.SceneComponent|GetRelativeLocation (Variables|Default|GetDoor)) "0,0,500.000000") "0, 0, 0" true true 3.0 false)
    (else
      (Development|PrintString "Buttons not Pressed"))))

(event EventDoorCodeLight3
  (Rendering|Components|Light|SetLightColor (Variables|Default|GetLight_3) (Utilities|Struct|MakeLinearColor 0.0 1.0 0.0 0.0) true)
  (bind _output_get (Variables|Default|SetLight_active_3 true))
  (if (Math|Boolean|ANDBoolean (stale EventDoorCodeLight1 _output_get) (stale EventDoorCodeLight2 _output_get) _output_get)
    (Components|MoveComponentTo (Variables|Default|GetDoor) (- (Variables|/Script/Engine.SceneComponent|GetRelativeLocation (Variables|Default|GetDoor)) "0,0,500.000000") "0, 0, 0" true true 3.0 false)
    (else
      (Development|PrintString "Buttons not Pressed"))))

(fn ConstructionScript)