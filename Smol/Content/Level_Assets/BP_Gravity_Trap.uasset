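; Gravity trap actor that pulls actors tagged Enemy (BP_Character_Enemy) toward its central sphere.
; Entering OuterPull stores the enemy in a single reference, turns off gravity and enables physics; Tick then adds velocity toward the sphere, scaled by distance and Acceleration.
; Reaching InnerPull or leaving OuterPull stops the pull and, after a short delay, zeroes velocity and disables capsule physics.
; Only leaving OuterPull restores gravity.
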(event OnComponentBeginOverlap(OuterPull)
  (params (OverlappedComponent :type Primitive%20Component%20Object%20Reference) (OtherActor :type Actor%20Object%20Reference) (OtherComp :type Primitive%20Component%20Object%20Reference) (OtherBodyIndex :type Integer) (bFromSweep :type Boolean) (SweepResult :type Hit%20Result%20Structure%20%28by%20ref%29))
  (if (Actor|ActorHasTag OtherActor "Enemy")
    (for _array_element (Utilities|Array|MakeArray OtherActor)
      (Development|PrintString "Enemy Overlapped(Outer pull)")
      (bind _asbp_character_enemy (Utilities|Casting|CastToBP_Character_Enemy OtherActor)
        (:then
          (bind _output_get (Variables|Default|SetEnemy_REF _asbp_character_enemy))
          (Physics|SetEnableGravity (Variables|/Game/Prototypes/Ina/BP_Character_Enemy.BP_Character_Enemy_C|GetCube _asbp_character_enemy) false)
          (Physics|SetSimulatePhysics (Variables|/Game/Prototypes/Ina/BP_Character_Enemy.BP_Character_Enemy_C|GetCube _asbp_character_enemy) true)
          (Development|PrintString "Gravity and Physics set")
          (Variables|Default|SetisAffectedbyGravity true))
        (:CastFailed
          (Development|PrintString "Enemy not found"))))))

(event OnComponentBeginOverlap(InnerPull)
  (params (OverlappedComponent :type Primitive%20Component%20Object%20Reference) (OtherActor :type Actor%20Object%20Reference) (OtherComp :type Primitive%20Component%20Object%20Reference) (OtherBodyIndex :type Integer) (bFromSweep :type Boolean) (SweepResult :type Hit%20Result%20Structure%20%28by%20ref%29))
  (if (Actor|ActorHasTag OtherActor "Enemy")
    (for _array_element (Utilities|Array|MakeArray OtherActor)
      (Variables|Default|SetisAffectedbyGravity false)
      (Development|PrintString "Enemy Overlapped(Inner pull)" false)
      (Utilities|FlowControl|Delay 0.2)
      (Variables|Default|SetVelocity "0, 0, 0")
      (Class|BPIGravity|ResetVelocity(Message) OtherActor)
      (bind _asbp_character_enemy (Utilities|Casting|CastToBP_Character_Enemy OtherActor))
      (Physics|SetPhysicsLinearVelocity (Variables|/Script/Engine.Character|GetCapsuleComponent _asbp_character_enemy) (Variables|Default|GetVelocity) false "None")
      (Physics|SetSimulatePhysics (Variables|/Script/Engine.Character|GetCapsuleComponent _asbp_character_enemy) false)
      (Components|Movement|StopMovementImmediately (Variables|/Script/Engine.Character|GetCharacterMovement _asbp_character_enemy))
      (Development|PrintString "End of Inner pull string" false true "(R=1.000000,G=0.050881,B=0.000000,A=1.000000)"))))

(event OnComponentEndOverlap(OuterPull)
  (params (OverlappedComponent :type Primitive%20Component%20Object%20Reference) (OtherActor :type Actor%20Object%20Reference) (OtherComp :type Primitive%20Component%20Object%20Reference) (OtherBodyIndex :type Integer))
  (if (Actor|ActorHasTag OtherActor "Enemy")
    (for _array_element (Utilities|Array|MakeArray OtherActor)
      (Variables|Default|SetisAffectedbyGravity false)
      (Development|PrintString "End overlap, Outerpull" false)
      (Utilities|FlowControl|Delay 0.2)
      (Variables|Default|SetVelocity "0, 0, 0")
      (Class|BPIGravity|ResetVelocity(Message) OtherActor)
      (bind _asbp_character_enemy (Utilities|Casting|CastToBP_Character_Enemy OtherActor))
      (Physics|SetPhysicsLinearVelocity (Variables|/Script/Engine.Character|GetCapsuleComponent _asbp_character_enemy) (Variables|Default|GetVelocity) false "None")
      (Physics|SetSimulatePhysics (Variables|/Script/Engine.Character|GetCapsuleComponent _asbp_character_enemy) false)
      (Physics|SetEnableGravity (Variables|/Game/Prototypes/Ina/BP_Character_Enemy.BP_Character_Enemy_C|GetCube _asbp_character_enemy) true)
      (Components|Movement|StopMovementImmediately (Variables|/Script/Engine.Character|GetCharacterMovement _asbp_character_enemy)))))

(event OnComponentEndOverlap(InnerPull)
  (params (OverlappedComponent :type Primitive%20Component%20Object%20Reference) (OtherActor :type Actor%20Object%20Reference) (OtherComp :type Primitive%20Component%20Object%20Reference) (OtherBodyIndex :type Integer)))

(event EventBeginPlay)

(event Collision|EventActorBeginOverlap
  (params (OtherActor :type Actor%20Object%20Reference)))

(event EventTick
  (params (DeltaSeconds :type Float%20%28single-precision%29))
  (if (Variables|Default|GetisAffectedbyGravity)
    (bind _output_get (Variables|Default|SetVelocity (* (* (- (Transformation|GetActorLocation (Variables|Default|GetEnemy_REF)) (Transformation|GetWorldLocation (Variables|Default|GetSphere))) (Variables|Default|GetAcceleration)) -1)))
    (Development|PrintString (Utilities|String|ToString(Vector) _output_get))
    (Physics|SetPhysicsLinearVelocity (Variables|/Script/Engine.Character|GetCapsuleComponent (stale OnComponentBeginOverlap(OuterPull) _asbp_character_enemy)) (Variables|Default|GetVelocity) true "None")))

(fn ConstructionScript)