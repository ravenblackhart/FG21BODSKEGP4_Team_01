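; BP_Pit_Tar is a tar pit hazard that slows the player while inside its Box volume.
; Begin and end overlap events drop the player's walk speed, then set it back to a hard-coded value rather than the previous one.
; Actors tagged "Enemy" are detected but only print a debug message after an empty loop; further speed-change and cast-failure nodes are left disconnected.
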(event OnComponentBeginOverlap(Box)
  (params (OverlappedComponent :type Primitive%20Component%20Object%20Reference) (OtherActor :type Actor%20Object%20Reference) (OtherComp :type Primitive%20Component%20Object%20Reference) (OtherBodyIndex :type Integer) (bFromSweep :type Boolean) (SweepResult :type Hit%20Result%20Structure%20%28by%20ref%29))
  (bind _returnvalue (Game|GetPlayerCharacter 0))
  (if (Class|KismetMathLibrary|XORBoolean (== OtherActor _returnvalue) (Actor|ActorHasTag OtherActor "Enemy"))
    (if (== OtherActor (Game|GetPlayerCharacter 0))
      (Variables|/Script/Engine.CharacterMovementComponent|SetMaxWalkSpeed (Variables|/Script/Engine.Character|GetCharacterMovement _returnvalue) 1e+02)
      (else
        ;[1 1 1] Enemy
        (Development|PrintString "Actor is Enemy")
        (for _array_element (Utilities|Array|MakeArray OtherActor)
          _)))
    (else
      (Development|PrintString "Not enemy or Player" true true "(R=1.000000,G=0.000000,B=0.129726,A=1.000000)"))))

(event OnComponentEndOverlap(Box)
  (params (OverlappedComponent :type Primitive%20Component%20Object%20Reference) (OtherActor :type Actor%20Object%20Reference) (OtherComp :type Primitive%20Component%20Object%20Reference) (OtherBodyIndex :type Integer))
  (bind _returnvalue (Game|GetPlayerCharacter 0))
  (if (Class|KismetMathLibrary|XORBoolean (== OtherActor (Game|GetPlayerCharacter 0)) (Actor|ActorHasTag OtherActor "Enemy"))
    (if (== OtherActor _returnvalue)
      (Variables|/Script/Engine.CharacterMovementComponent|SetMaxWalkSpeed (Variables|/Script/Engine.Character|GetCharacterMovement _returnvalue) 5e+02)
      (else
        ;[1 1 1] Enemy
        (Development|PrintString "Actor is Enemy")
        (for _array_element (Utilities|Array|MakeArray OtherActor)
          _)))))

(fn ConstructionScript)