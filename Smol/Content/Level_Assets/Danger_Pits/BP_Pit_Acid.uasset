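; BP_Pit_Acid is an acid pit hazard that kills the player and slows enemies on contact.
; Its box overlap accepts the first player character or actors tagged Enemy.
; For the player, it zeroes PlayerHealth in GI_SMOL and triggers the health check.
; BP_Character_Enemy_1 instances get a permanently lowered walk speed, with debug prints apparently carried over from a tar pit.
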(event OnComponentBeginOverlap(Box)
  (params (OverlappedComponent :type Primitive%20Component%20Object%20Reference) (OtherActor :type Actor%20Object%20Reference) (OtherComp :type Primitive%20Component%20Object%20Reference) (OtherBodyIndex :type Integer) (bFromSweep :type Boolean) (SweepResult :type Hit%20Result%20Structure%20%28by%20ref%29))
  (if (Class|KismetMathLibrary|XORBoolean (== OtherActor (Game|GetPlayerCharacter 0)) (Actor|ActorHasTag OtherActor "Enemy"))
    (if (== OtherActor (Game|GetPlayerCharacter 0))
      ;[1 1 1] Player hit by pit
      (bind _asgi_smol (Utilities|Casting|CastToGI_SMOL (Game|GetGameInstance)))
      (Variables|/Game/GI_SMOL.GI_SMOL_C|SetPlayer_Health _asgi_smol 0)
      (Class|BPIStats|PlayerCheckHealth(Message) _asgi_smol)
      (Development|PrintString "Health check from Acid" true true "(R=1.000000,G=0.996317,B=0.985269,A=1.000000)")
      (Utilities|FlowControl|Delay 1.0)
      (else
        ;[1 1 1] Enemy hit by Pit
        (Development|PrintString "Actor is Enemy")
        (for _array_element (Utilities|Array|MakeArray OtherActor)
          (bind _asbp_character_enemy_1 (Utilities|Casting|CastToBP_Character_Enemy_1 _array_element)
            (:then
              (Development|PrintString "Cast complete")
              (Variables|/Script/Engine.CharacterMovementComponent|SetMaxWalkSpeed (Variables|/Script/Engine.Character|GetCharacterMovement _asbp_character_enemy_1) 1e+02))
            (:CastFailed
              (Development|PrintString "Cast failed to Enemy (Pit_Tar)" true true "(R=1.000000,G=0.661424,B=0.000000,A=1.000000)"))))))))

(fn ConstructionScript)