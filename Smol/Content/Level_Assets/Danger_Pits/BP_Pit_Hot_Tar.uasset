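; Hot tar pit hazard that slows the player and drains health while they stand inside its Box trigger.
; Entering sets a damage flag and starts a Delay loop that subtracts Damage from GI_SMOL's PlayerHealth every 1.5 seconds and requests a health check.
; Leaving restores a hardcoded walk speed and clears the flag to end the loop.
; Enemy-tagged actors only trigger debug prints; their slow and damage logic is disconnected.
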(event OnComponentEndOverlap(Box)
  (params (OverlappedComponent :type Primitive%20Component%20Object%20Reference) (OtherActor :type Actor%20Object%20Reference) (OtherComp :type Primitive%20Component%20Object%20Reference) (OtherBodyIndex :type Integer))
  (bind _returnvalue (Game|GetPlayerCharacter 0))
  ;[1 1 1] Stop damage
  (if (Class|KismetMathLibrary|XORBoolean (== OtherActor _returnvalue) (Actor|ActorHasTag OtherActor "Enemy"))
    (if (== OtherActor (Game|GetPlayerCharacter 0))
      (Variables|/Script/Engine.CharacterMovementComponent|SetMaxWalkSpeed (Variables|/Script/Engine.Character|GetCharacterMovement _returnvalue) 5e+02)
      (Variables|Default|SetDealDamage false)
      (else
        (Development|PrintString "Actor is Enemy")
        (for _array_element (Utilities|Array|MakeArray OtherActor)
          _)))))

(event OnComponentBeginOverlap(Box)
  (params (OverlappedComponent :type Primitive%20Component%20Object%20Reference) (OtherActor :type Actor%20Object%20Reference) (OtherComp :type Primitive%20Component%20Object%20Reference) (OtherBodyIndex :type Integer) (bFromSweep :type Boolean) (SweepResult :type Hit%20Result%20Structure%20%28by%20ref%29))
  (bind _returnvalue (Game|GetPlayerCharacter 0))
  (if (Class|KismetMathLibrary|XORBoolean (== OtherActor _returnvalue) (Actor|ActorHasTag OtherActor "Enemy"))
    (if (== OtherActor (Game|GetPlayerCharacter 0))
      (Variables|Default|SetDealDamage true)
      (Variables|/Script/Engine.CharacterMovementComponent|SetMaxWalkSpeed (Variables|/Script/Engine.Character|GetCharacterMovement _returnvalue) 1e+02)
      (if (Variables|Default|GetDealDamage) :!label _label
        ;[1 1 1] Player Damaged by pit
        (bind _asgi_smol (Utilities|Casting|CastToGI_SMOL (Game|GetGameInstance)))
        (Variables|/Game/GI_SMOL.GI_SMOL_C|SetPlayer_Health _asgi_smol (- (Variables|/Game/GI_SMOL.GI_SMOL_C|GetPlayer_Health _asgi_smol) (Variables|Default|GetDamage)))
        (Class|BPIStats|PlayerCheckHealth(Message) _asgi_smol)
        (Development|PrintString "Health check from Acid" true true "(R=1.000000,G=0.996317,B=0.985269,A=1.000000)")
        (Utilities|FlowControl|Delay 1.0)
        (Utilities|FlowControl|Delay 0.5)
        (goto _label))
      (else
        (Development|PrintString "Actor is Enemy")))))

(fn ConstructionScript)